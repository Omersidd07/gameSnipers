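; Sniper weapon Blueprint that overrides the firing and reload events of a parent weapon class.
; While bullets remain, InternalShoot spawns a BP_MachineGunProjectile at the ShootingDir transform, assigned the weapon's owner, then decrements the count and plays a rifle fire sound.
; ReloadWeapon plays a reload sound and defers to the parent's logic.
; Weapon mesh animation nodes for firing and reloading are present but never run.
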(event EventBeginPlay
  (|CallParentFunction) ; This node is disabled and will not be called.\nDrag off pins to build functionality.
)

(event Collision|EventActorBeginOverlap
  (params (OtherActor :type Actor%20Object%20Reference))
  (|CallParentFunction OtherActor) ; This node is disabled and will not be called.\nDrag off pins to build functionality.
)

(event EventTick
  (params (DeltaSeconds :type Float%20%28single-precision%29))
  (|CallParentFunction DeltaSeconds) ; This node is disabled and will not be called.\nDrag off pins to build functionality.
)

(event EventReloadWeapon
  (Audio|PlaySoundatLocation "/Game/MilitaryWeapSilver/Sound/Rifle/Wavs/Rifle_Reload01.Rifle_Reload01" (Transformation|GetWorldLocation (Variables|Default|GetDefaultSceneRoot)) "0, 0, 0" 1.0 1.0 0.0 0 0 0 0)
  (|CallParentFunction))

(event EventInternalShoot
  (if (not (<= (Variables|Default|GetNumBullets) 0))
    (Game|SpawnActorfromClass "/Game/Projectile/BP_MachineGunProjectile.BP_MachineGunProjectile_C" (Transformation|GetWorldTransform (Variables|Default|GetShootingDir)) "AlwaysSpawn" "MultiplyWithRoot" (Components|GetOwner) 0)
    (Variables|Default|SetNumBullets (- (Variables|Default|GetNumBullets) 1))
    (Audio|PlaySoundatLocation "/Game/MilitaryWeapSilver/Sound/Rifle/Wavs/RifleA_Fire01.RifleA_Fire01" (Transformation|GetWorldLocation (Variables|Default|GetDefaultSceneRoot)) "0, 0, 0" 1.0 1.0 0.0 0 0 0 0)))

(fn ConstructionScript
  (|CallParentFunction))